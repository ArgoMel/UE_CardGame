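; Physics die actor that rolls itself and records a 1–6 result in SayiInt.
; Salla applies a random rotation and impulse, disables the six face boxes' collision, then polls location every 0.2 seconds until the die stops moving.
; At rest it sets Durdu and re-enables the boxes, whose overlaps with the floor reference set the number.
; BeginPlay assigns None to that floor reference.
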(event OnComponentBeginOverlap(Box1)
  (params (OverlappedComponent :type Primitive%20Component%20Object%20Reference) (OtherActor :type Actor%20Object%20Reference) (OtherComp :type Primitive%20Component%20Object%20Reference) (OtherBodyIndex :type Integer) (bFromSweep :type Boolean) (SweepResult :type Hit%20Result%20Structure%20%28by%20ref%29))
  (if (== OtherActor (.As%20Floor%20Blueprint%20ref (Variables|Default|GetAs%20Floor%20Blueprint%20ref)))
    (Variables|Default|Setsayi_int 1)))

(event OnComponentBeginOverlap(Box6)
  (params (OverlappedComponent :type Primitive%20Component%20Object%20Reference) (OtherActor :type Actor%20Object%20Reference) (OtherComp :type Primitive%20Component%20Object%20Reference) (OtherBodyIndex :type Integer) (bFromSweep :type Boolean) (SweepResult :type Hit%20Result%20Structure%20%28by%20ref%29))
  (if (== OtherActor (.As%20Floor%20Blueprint%20ref (Variables|Default|GetAs%20Floor%20Blueprint%20ref)))
    (Variables|Default|Setsayi_int 6)))

(event OnComponentBeginOverlap(Box5)
  (params (OverlappedComponent :type Primitive%20Component%20Object%20Reference) (OtherActor :type Actor%20Object%20Reference) (OtherComp :type Primitive%20Component%20Object%20Reference) (OtherBodyIndex :type Integer) (bFromSweep :type Boolean) (SweepResult :type Hit%20Result%20Structure%20%28by%20ref%29))
  (if (== OtherActor (.As%20Floor%20Blueprint%20ref (Variables|Default|GetAs%20Floor%20Blueprint%20ref)))
    (Variables|Default|Setsayi_int 5)))

(event OnComponentBeginOverlap(Box2)
  (params (OverlappedComponent :type Primitive%20Component%20Object%20Reference) (OtherActor :type Actor%20Object%20Reference) (OtherComp :type Primitive%20Component%20Object%20Reference) (OtherBodyIndex :type Integer) (bFromSweep :type Boolean) (SweepResult :type Hit%20Result%20Structure%20%28by%20ref%29))
  (if (== OtherActor (.As%20Floor%20Blueprint%20ref (Variables|Default|GetAs%20Floor%20Blueprint%20ref)))
    (Variables|Default|Setsayi_int 2)))

(event OnComponentBeginOverlap(Box3)
  (params (OverlappedComponent :type Primitive%20Component%20Object%20Reference) (OtherActor :type Actor%20Object%20Reference) (OtherComp :type Primitive%20Component%20Object%20Reference) (OtherBodyIndex :type Integer) (bFromSweep :type Boolean) (SweepResult :type Hit%20Result%20Structure%20%28by%20ref%29))
  (if (== OtherActor (.As%20Floor%20Blueprint%20ref (Variables|Default|GetAs%20Floor%20Blueprint%20ref)))
    (Variables|Default|Setsayi_int 3)))

(event OnComponentBeginOverlap(Box4)
  (params (OverlappedComponent :type Primitive%20Component%20Object%20Reference) (OtherActor :type Actor%20Object%20Reference) (OtherComp :type Primitive%20Component%20Object%20Reference) (OtherBodyIndex :type Integer) (bFromSweep :type Boolean) (SweepResult :type Hit%20Result%20Structure%20%28by%20ref%29))
  (if (== OtherActor (.As%20Floor%20Blueprint%20ref (Variables|Default|GetAs%20Floor%20Blueprint%20ref)))
    (Variables|Default|Setsayi_int 4)))

(event Custom|Is%20moving?
  (Variables|Default|SetLocation_var (Transformation|GetActorLocation))
  (Utilities|FlowControl|Delay 0.2)
  (if (Math|Vector|Equal(Vector) (Variables|Default|GetLocation_var) (Transformation|GetActorLocation) 0.0001)
    (Development|PrintString "Durdu")
    (Variables|Default|SetDurdu true)
    (Collision|SetCollisionEnabled (Variables|Default|GetBox1) "QueryAndPhysics")
    (else
      (CallFunction|IsMoving?))))

(event Custom|Salla
  (bind _returnvalue (Math|Random|RandomFloatinRange -3.6e+02 3.6e+02))
  (bind _returnvalue_2 (Math|Random|RandomFloatinRange -3.6e+02 3.6e+02))
  (bind _returnvalue_3 (Math|Random|RandomFloatinRange -3.6e+02 3.6e+02))
  (Variables|Default|SetDurdu false)
  (Transformation|SetActorRotation (Math|Rotator|MakeRotator _returnvalue_2 _returnvalue_3 _returnvalue))
  (Physics|AddImpulse (Variables|Debug|GetStaticMeshComponent) (Math|Vector|MakeVector (* _returnvalue_2 1e+01) (* _returnvalue_3 1e+01) (* _returnvalue 1e+01)) "None" false)
  (CallFunction|IsMoving?)
  (Collision|SetCollisionEnabled (Variables|Default|GetBox1) "NoCollision"))

(event EventBeginPlay
  (bind _as액터 (Utilities|Casting|CastToActorClass 0))
  (bind _returnvalue (Actor|GetActorOfClass _as액터))
  (bind _asfloor_blueprint (Utilities|Casting|CastTo _returnvalue))
  (Variables|Default|SetAs%20Floor%20Blueprint%20ref 0 _asfloor_blueprint))

(fn ConstructionScript)