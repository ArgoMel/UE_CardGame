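; Blueprint function library of shared helpers for the game's card system.
; GetRandomCard picks a random row name from the DT_CardInfo data table and returns that card's row.
; InterpolateTowardsLoc eases a widget transform toward a destination by interpolating translation and angle with a given speed and delta time, leaving other transform components at their defaults.
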(fn GetRandomCard
  (bind _outrownames (DataTable|GetDataTableRowNames "/Game/Card/Data/DT_CardInfo.DT_CardInfo"))
  (bind _returnvalue (Utilities|GetDataTableRow "/Game/Card/Data/DT_CardInfo.DT_CardInfo" (.OutItem (Utilities|Array|Random _outrownames)))
    (:then
      (return _returnvalue))))

(fn InterpolateTowardsLoc
  (params (CurTransform :type Widget%20Transform%20Structure) (DestTransform :type Widget%20Transform%20Structure) (DeltaTime :type Float%20%28double-precision%29) (InterpolationSpeed :type Float%20%28double-precision%29))
  (bind (_translation _scale _shear _angle) (Utilities|Struct|BreakWidgetTransform CurTransform))
  (bind (_translation_2 _scale_2 _shear_2 _angle_2) (Utilities|Struct|BreakWidgetTransform DestTransform))
  (return (Utilities|Struct|MakeWidgetTransform (Class|KismetMathLibrary|Vector2DInterpto _translation _translation_2 DeltaTime InterpolationSpeed) "(X=1.000000,Y=1.000000)" "(X=0.000000,Y=0.000000)" (Math|Interpolation|FInterpTo _angle _angle_2 DeltaTime InterpolationSpeed))))